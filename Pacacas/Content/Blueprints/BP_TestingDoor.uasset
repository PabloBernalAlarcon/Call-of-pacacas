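; BP_TestingDoor is a test door actor that prints a debug message and calls OpenDoor on BeginPlay.
; OpenDoor is not defined in this graph, while the BP_OpenDoor and BP_CloseDoor events snap the Door component's relative yaw with no interpolation.
; Both events set the yaw to DoorOpenAngle, so BP_CloseDoor applies the same rotation as opening.
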(event Custom|BP_CloseDoor
  (Transformation|SetRelativeRotation (Variables|Default|GetDoor) (Math|Rotator|MakeRotator 0.0 0.0 (Variables|Default|GetDoorOpenAngle)) false false))

(event Custom|BP_OpenDoor
  (Transformation|SetRelativeRotation (Variables|Default|GetDoor) (Math|Rotator|MakeRotator 0.0 0.0 (Variables|Default|GetDoorOpenAngle)) false false))

(event EventBeginPlay
  (Development|PrintString "Amen🙏🙏🙏" true true "(R=0.873923,G=0.199000,B=1.000000,A=1.000000)" 5.0)
  (CallFunction|OpenDoor))

(event Collision|EventActorBeginOverlap
  (params (OtherActor :type Actor%20Object%20Reference)))

(event EventTick
  (params (DeltaSeconds :type Float%20%28single-precision%29)))

(fn ConstructionScript)